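; BP_Button is a button actor that responds to a player interaction, currently only by printing debug text.
; The INTAction event stores the passed Player, then prints "Yes" or "NO" depending on an overlap flag.
; Box begin and end overlap events set and clear that flag when the other actor matches the stored Player, a reference this graph assigns only in INTAction.
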(event `/Game/ThirdPerson/Blueprints/BPI_Interaction.INT_Action`
  (params (` Player` :type "Actor Object Reference"))
  (set `self.Player` ` Player`)
  (if (`self.isOverlapingPlayer?`)
    (`KismetSystemLibrary.PrintString` "Yes" true true (struct :`G` 0.66 :`B` 1.0 :`A` 1.0) 2.0 "Yes I")
    (else
      (`KismetSystemLibrary.PrintString` "NO" true true (struct :`G` 0.66 :`B` 1.0 :`A` 1.0) 2.0 "NO I"))))

(event `self.Box.OnComponentBeginOverlap`
  (params (OverlappedComponent :type "PrimitiveComponent Object Reference") (OtherActor :type "Actor Object Reference") (OtherComp :type "PrimitiveComponent Object Reference") (OtherBodyIndex :type Integer) (bFromSweep :type Boolean) (SweepResult :type "HitResult Structure (by ref)"))
  (if (== OtherActor (`self.Player`))
    (set `self.isOverlapingPlayer?` true)))

(event `self.Box.OnComponentEndOverlap`
  (params (OverlappedComponent :type "PrimitiveComponent Object Reference") (OtherActor :type "Actor Object Reference") (OtherComp :type "PrimitiveComponent Object Reference") (OtherBodyIndex :type Integer))
  (if (== OtherActor (`self.Player`))
    (set `self.isOverlapingPlayer?` false)))

(fn `UserConstructionScript`)