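; Boss enemy Blueprint that adds a special attack on top of inherited behavior.
; Its SpecialAttack event clears the SpecialAttack flag on the controller's Blackboard, calls Attack, then sets the flag back to true after a short delay.
; BeginPlay, overlap and Tick are disabled stubs, and the construction script only calls the parent.
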(event `SpecialAttack`
  (`BlackboardComponent.SetValueAsBool` (`AIBlueprintHelperLibrary.GetBlackboard` (`self.GetController`)) (`self.Special Attack`) false)
  (`self.Attack`)
  (`KismetSystemLibrary.Delay` 0.2)
  (`BlackboardComponent.SetValueAsBool` (`AIBlueprintHelperLibrary.GetBlackboard` (`self.GetController`)) (`self.Special Attack`) true))

(fn `UserConstructionScript`
  (`parent.UserConstructionScript`))