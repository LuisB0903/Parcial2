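; BP_DamageText is a short-lived actor that displays a damage value through a widget component.
; On BeginPlay it passes Damage to the widget and derives an end point offset upward and diagonally from its spawn location.
; The Move timeline sets the location from a lerp between both points, though Alpha shows as a constant zero, then destroys the actor when finished.
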(event `self.ReceiveBeginPlay`
  (message `/Game/Interfaces/BPI_WeaponHolder.Update Damage HUD` (`WidgetComponent.GetWidget` (`self.Widget`)) (`self.Damage`))
  (bind _output_get (set `self.Start` (`self.K2_GetActorLocation`)))
  (set `self.End` (+ _output_get (-25.0 -25.0 100.0)))
  (`Timeline|Move`
    (:`Update`
      (`self.K2_SetActorLocation` (`KismetMathLibrary.VLerp` (`self.Start`) (`self.End`))))
    (:`Finished`
      (`self.K2_DestroyActor`))))

(fn `UserConstructionScript`)