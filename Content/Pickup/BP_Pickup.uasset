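; Respawning weapon pickup that hands its weapon class to an overlapping actor tagged Player.
; BeginPlay reads a data table row and async-loads the mesh and weapon class.
; Tick calls Spin to bob and rotate the mesh from game time.
; On pickup it hides and disables collision and tick until a timer replays it through a scale-in timeline, restoring both when finished.
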(event `self.ReceiveBeginPlay`
  (bind (_datatable _rowname) (break `DataTableRowHandle` (`self.WeaponType`)))
  (bind (_relativelocation_x _relativelocation_y _relativelocation_z) (`KismetMathLibrary.BreakVector` (`SceneComponent.RelativeLocation` (`self.StaticMesh`))))
  ;[0.15 0.07477 0 0.5] Spawn
  (set `self.RelativeLocationZ` _relativelocation_z)
  (bind _returnvalue (`|GetDataTableRow` _datatable _rowname)
    (:`then`
      (`|ExecutionSequence`
        (:`then_0`
          (bind (_staticmesh _weaponclass) (break `/Game/Pickup/ST_WeaponTable` _returnvalue))
          (bind _object (`|LoadAsset` _staticmesh)
            (:`Completed`
              (`StaticMeshComponent.SetStaticMesh` (`self.StaticMesh`) (cast `StaticMesh` _object :!pure true)))))
        (:`then_1`
          (bind _class (`|LoadAssetClass` _weaponclass)
            (:`Completed`
              (bind _asbp_weapon_base (castclass `/Game/Pickup/Weapons/BP_WeaponBase` _class))
              (set `self.WeaponClass` _asbp_weapon_base))))))))

(event `self.ReceiveTick`
  (params (DeltaSeconds :type "Float (single-precision)"))
  ;[0.005192 0.1318 0.15 0.5] Tick
  (`self.Spin` (0.5 0.5 0.5)))

(event `self.Sphere.OnComponentBeginOverlap`
  (params (OverlappedComponent :type "PrimitiveComponent Object Reference") (OtherActor :type "Actor Object Reference") (OtherComp :type "PrimitiveComponent Object Reference") (OtherBodyIndex :type Integer) (bFromSweep :type Boolean) (SweepResult :type "HitResult Structure (by ref)"))
  (if (`self.ActorHasTag` OtherActor "Player")
    (message `/Game/Pickup/BPI_WeaponHolder.Add Weapon Class` OtherActor (`self.WeaponClass`))
    (`SceneComponent.SetHiddenInGame` (`self.StaticMesh`) true false)
    (`PrimitiveComponent.SetCollisionEnabled` (`self.Sphere`) "NoCollision")
    (`self.SetActorTickEnabled` false)
    (`KismetSystemLibrary.K2_SetTimerDelegate` (delegate `Enable Pickup`) (`self.SpawnTime`))))

(event `Enable Pickup`
  (`SceneComponent.SetHiddenInGame` (`self.StaticMesh`) false false)
  (bind (_direction _scalein) (`Timeline|Spawnin` :!via `PlayFromStart`)
    (:`Update`
      (`self.Spin` (`KismetMathLibrary.Conv_DoubleToVector` _scalein)))
    (:`Finished`
      (`PrimitiveComponent.SetCollisionEnabled` (`self.Sphere`) "QueryOnly")
      (`self.SetActorTickEnabled` true))))

(fn `Spin`
  (params (Scale :type "Vector Structure"))
  (bind _returnvalue (`KismetSystemLibrary.GetGameTimeInSeconds`))
  (`SceneComponent.K2_SetRelativeTransform` (`self.StaticMesh`) (`KismetMathLibrary.MakeTransform` (`KismetMathLibrary.MakeVector` 0.0 0.0 (+ (`self.RelativeLocationZ`) (`KismetMathLibrary.Sin` (* _returnvalue 5.0)))) (`KismetMathLibrary.MakeRotator` 0.0 0.0 (* _returnvalue 100.0)) Scale) false false))

(fn `UserConstructionScript`)